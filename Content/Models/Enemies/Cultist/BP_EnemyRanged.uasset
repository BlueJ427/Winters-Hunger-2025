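; BP_EnemyRanged is a ranged enemy that fires a rifle to deal sanity damage to the player.
; On BeginPlay it spawns a rifle and attaches it to the mesh's weapon socket.
; Attack plays the fire montage, whose notify traces from the weapon to the AI controller's target and damages sanity only if nothing blocks it.
; It signals attack end when the montage finishes and supplies its ideal attack and defend ranges.
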(event `self.ReceiveBeginPlay`
  (`/Game/Models/Enemies/Cultist/AI/BPI_EnemyAI.EquipWeapon`))

(event `/Game/Models/Enemies/Cultist/AI/BPI_EnemyAI.EquipWeapon`
  (bind _returnvalue (`|SpawnActorFromClass` "/Game/Models/Weapons/Rifle/BP_Weapon_Rifle.BP_Weapon_Rifle_C" (`KismetMathLibrary.MakeTransform` (0.0 0.0 0.0)) "Undefined" "MultiplyWithRoot" null null))
  (bind _output_get (set `self.WeaponActor` _returnvalue))
  (bind _returnvalue_2 (`self.K2_AttachToComponent` _output_get (`self.Mesh`) "WeaponBone" "SnapToTarget" "SnapToTarget" "SnapToTarget" true))
  (set `self.IsWieldingWeapon` _returnvalue_2))

(event `/Game/Models/Enemies/Cultist/AI/BPI_EnemyAI.Attack`
  (bind _notifyname (`|PlayMontage` (`self.Mesh`) "/Game/Models/Enemies/Cultist/Anim/Montage_Rifle_Fire.Montage_Rifle_Fire")
    (:`OnCompleted`
      (`self.OnAttackEnd` :!label _label))
    (:`OnInterrupted`
      (goto _label))
    (:`OnNotifyBegin`
      (switch `name` _notifyname
        (:`Fire`
          (bind _asaic_enemy_base (cast `/Game/Models/Enemies/Cultist/AI/AIC_EnemyBase` (`AIBlueprintHelperLibrary.GetAIController` self)))
          (bind _attack_target (`/Game/Models/Enemies/Cultist/AI/AIC_EnemyBase.Attack Target` _asaic_enemy_base)
            (:`then`
              (bind (_outhit _returnvalue) (`KismetSystemLibrary.LineTraceSingle` :`Start` (`self.K2_GetActorLocation` (`self.WeaponActor`)) :`End` (`self.K2_GetActorLocation` _attack_target) :`TraceChannel` "TraceTypeQuery1" :`DrawDebugType` "ForDuration" :`TraceColor` (struct :`G` 1.0 :`B` 0.008223 :`A` 1.0) :`TraceHitColor` (struct :`R` 1.0 :`B` 0.087291 :`A` 1.0)))
              (if (not _returnvalue)
                (bind _asbp_player (cast `/Game/Blueprints/BP_Player` _attack_target))
                (`/Game/Blueprints/BP_Player.Sanity Damage` _asbp_player 10.0)))
            (:`else`)))))))

(fn `GetIdealRange`
  (returns (AttackRadius :type "Float (double-precision)") (DefendRadius :type "Float (double-precision)"))
  (return 600.0 600.0))

(fn `UserConstructionScript`
  (`parent.UserConstructionScript`))