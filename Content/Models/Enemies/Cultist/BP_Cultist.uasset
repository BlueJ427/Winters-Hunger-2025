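; BP_Cultist is an enemy character with health, weapon wielding and functions for attack, range, patrol and speed queries.
; Attack is a placeholder that prints a message, then fires OnAttackEnd after a short delay.
; EquipWeapon spawns and socket-attaches a base weapon, damage lowers clamped health until flagged dead, and SetMovementSpeed maps movement states to walk speeds.
; GetIdealRange and GetPatrolRoute are stubs returning zero or empty values.
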(event `self.ReceiveBeginPlay`)

(event `/Game/Models/Enemies/Cultist/AI/BPI_EnemyAI.Attack`
  (`KismetSystemLibrary.PrintString` "I've hurt the player!")
  (`KismetSystemLibrary.Delay` 0.2)
  (`self.OnAttackEnd`))

(event `/Game/Models/Enemies/Cultist/AI/BPI_EnemyAI.EquipWeapon`
  (bind _returnvalue (`|SpawnActorFromClass` "/Game/Models/Weapons/Rifle/BP_Weapon_Base.BP_Weapon_Base_C" (`self.GetTransform`) "Undefined" "MultiplyWithRoot" null null))
  (bind _output_get (set `self.WeaponActor` _returnvalue))
  (`self.K2_AttachToComponent` _output_get (`self.Mesh`) "WeaponBone" "SnapToTarget" "SnapToTarget" "SnapToTarget" true)
  (set `self.IsWieldingWeapon` true))

(event `self.ReceiveAnyDamage`
  (params (Damage :type "Float (single-precision)") (DamageType :type "DamageType Object Reference") (InstigatedBy :type "Controller Object Reference") (DamageCauser :type "Actor Object Reference"))
  (bind _output_get (set `self.Health` (`KismetMathLibrary.FClamp` (- (`self.Health`) Damage) 0.0 (`self.MaxHealth`))))
  (if (<= _output_get 0.0)
    (set `self.isDead` true)))

(fn `GetIdealRange`
  (returns (AttackRadius :type "Float (double-precision)") (DefendRadius :type "Float (double-precision)"))
  (return 0.0 0.0))

(fn `GetPatrolRoute`
  (returns (PatrolRoute :type "/Game/Models/Enemies/Cultist/AI/BP_PatrolRoute Object Reference"))
  (return null))

(fn `SetMovementSpeed`
  (params (Speed :type "/Game/Models/Enemies/Cultist/AI/Enum/E_MovementSpeed Enum" :default "NewEnumerator0"))
  (returns (SpeedValue :type "Float (double-precision)"))
  (set `CharacterMovementComponent.MaxWalkSpeed` (select `/Game/Models/Enemies/Cultist/AI/Enum/E_MovementSpeed` Speed :`NewEnumerator1` 200.0 :`NewEnumerator2` 300.0 :!type "Float (single-precision)") (`self.CharacterMovement`))
  (return 0.0))

(fn `UserConstructionScript`)