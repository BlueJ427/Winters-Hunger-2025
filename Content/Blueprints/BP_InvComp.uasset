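; Inventory component that holds a fixed-size array of item structs and displays it through a WB_Inventory widget created at BeginPlay.
; The inventory input action toggles the widget, mouse cursor and input mode.
; A camera line-trace pickup that stacks matching items or fills empty slots, refreshes the widget and destroys the item actor is present but disconnected, so the interact input does nothing.
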(event `self.ReceiveBeginPlay`
  (bind _returnvalue (`|CreateWidget` "/Game/HUD/Inventory/WB_Inventory.WB_Inventory_C"))
  (set `self.Inventory Widget` _returnvalue)
  (`KismetArrayLibrary.Array_Resize` (`self.Items`) 10)
  (`/Game/HUD/Inventory/WB_Inventory.LoadInv` (`self.Inventory Widget`) self))

(event `EnhancedInput|/Game/Blueprints/Input/IA_Inv`
  (params (ActionValue :type Boolean) (ElapsedSeconds :type "Float (double-precision)") (TriggeredSeconds :type "Float (double-precision)") (InputAction :type "InputAction Object Reference" :default "/Game/Blueprints/Input/IA_Inv.IA_Inv"))
  (bind _returnvalue (`GameplayStatics.GetPlayerController` 0))
  (bind _returnvalue_2 (`GameplayStatics.GetPlayerController` 0))
  (bind _inventory_widget (`self.Inventory Widget`))
  (:`Started`
    (if (`Widget.IsVisible` _inventory_widget)
      (`Widget.RemoveFromParent` _inventory_widget)
      (set `PlayerController.bShowMouseCursor` false _returnvalue)
      (`WidgetBlueprintLibrary.SetInputMode_GameOnly` _returnvalue)
      (else
        (set `PlayerController.bShowMouseCursor` true _returnvalue_2)
        (`WidgetBlueprintLibrary.SetInputMode_GameAndUIEx` _returnvalue_2 null)
        (`UserWidget.AddToViewport` _inventory_widget 0)))))

(event `EnhancedInput|/Game/Blueprints/Input/IA_Interact`
  (params (ActionValue :type Boolean) (ElapsedSeconds :type "Float (double-precision)") (TriggeredSeconds :type "Float (double-precision)") (InputAction :type "InputAction Object Reference" :default "/Game/Blueprints/Input/IA_Interact.IA_Interact")))