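; BP_ExtraItem is an interactable item actor whose construction script sets its static mesh from its Item data.
; StartInteract acts only when the StaticMesh component's display name, rather than the mesh asset's, contains "Campfire".
; It then plays three attenuated campfire sounds attached to the mesh in a delayed sequence, with a DoOnce blocking retriggers until the final delay ends.
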(event `/Game/Blueprints/BPI_Interact.StartInteract`
  (params (PlayerCharacter :type "/Game/Blueprints/BP_Player Object Reference"))
  (if (`KismetStringLibrary.Contains` (`KismetSystemLibrary.GetDisplayName` (`self.StaticMesh`)) "Campfire")
    (`/Engine/EditorBlueprintResources/StandardMacros.DoOnce` false :!label _label
      (:`Completed`
        (`GameplayStatics.SpawnSoundAttached` "/Game/Audio/SFX/Nightmare_Works_(Capstone)/Environment_Sounds/Individual_Sounds/CampFire.CampFire" (`self.StaticMesh`) "None" (0.0 0.0 0.0) (struct) "KeepRelativeOffset" false 1.0 1.0 0.0 "/Game/Audio/MediumDistanceSoundAttenuation.MediumDistanceSoundAttenuation" null)
        (`KismetSystemLibrary.Delay` 13.0)
        (`GameplayStatics.SpawnSoundAttached` "/Game/Audio/SFX/Nightmare_Works_(Capstone)/Environment_Sounds/Individual_Sounds/CampFire_2.CampFire_2" (`self.StaticMesh`) "None" (0.0 0.0 0.0) (struct) "KeepRelativeOffset" false 1.0 1.0 0.0 "/Game/Audio/MediumDistanceSoundAttenuation.MediumDistanceSoundAttenuation" null)
        (`KismetSystemLibrary.Delay` 7.0)
        (`GameplayStatics.SpawnSoundAttached` "/Game/Audio/SFX/Nightmare_Works_(Capstone)/Environment_Sounds/Individual_Sounds/Campfire_3_.Campfire_3_" (`self.StaticMesh`) "None" (0.0 0.0 0.0) (struct) "KeepRelativeOffset" false 1.0 1.0 0.0 "/Game/Audio/MediumDistanceSoundAttenuation.MediumDistanceSoundAttenuation" null)
        (`KismetSystemLibrary.Delay` 7.0)
        (goto _label :!via `Reset`)))))

(fn `UserConstructionScript`
  (`StaticMeshComponent.SetStaticMesh` (`self.StaticMesh`) (`.Mesh_14_BE31C94F4C13F0E4B082E4BA04368C96` (break `/Game/Blueprints/Inventory/S_ItemStruct` (`self.Item`)))))