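; AI_Cultist is an enemy that patrols waypoints and attacks the player's sanity, apparently adapted from a wolf AI.
; A looping ProcessArray event uses AIMoveTo through the Waypoints, with a small random chance on each arrival to chase the player instead, without any sight check.
; On reaching the player, a forward sphere trace must hit BP_Player to decrease sanity and resume patrol.
; StartShot destroys the actor; wolf sound nodes are disconnected.
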(event `self.ReceiveBeginPlay`
  (bind _output_get (set `self.LastIndex` (`KismetArrayLibrary.Array_LastIndex` (`self.Waypoints`))))
  (bind _result (`/Engine/EditorBlueprintResources/StandardMacros.IncrementInt` _output_get)
    (:`  `
      (set `self.LastIndex` _result)
      (`self.Process Array`))))

(event `self.ReceiveTick`
  (params (DeltaSeconds :type "Float (single-precision)")))

(event `Process Array`
  (bind _returnvalue (`self.K2_GetActorLocation`))
  (bind _waypoints (`self.Waypoints`))
  (bind _currentwaypoint (`self.CurrentWayPoint`))
  ;[1 1 1] Wolf moving using waypoints, if it spots player it will target and attack before returning to waypoint
  (`|AIMoveTo` self (`self.K2_GetActorLocation` (`|GetArrayItem` _waypoints _currentwaypoint)) null 1.0
    (:`OnSuccess`
      (if (`KismetMathLibrary.RandomBoolWithWeight` 0.1)
        (`|AIMoveTo` self (0.0 0.0 0.0) (`GameplayStatics.GetPlayerCharacter` 0) 1.0
          (:`OnSuccess`
            (`KismetSystemLibrary.PrintString` "Attack")
            (bind _outhit (`KismetSystemLibrary.SphereTraceSingleForObjects` _returnvalue (+ _returnvalue (* (`KismetMathLibrary.GetForwardVector` (`self.K2_GetActorRotation`)) 500.0)) 350.0 (`|MakeArray` "ObjectTypeQuery3" :!type "EObjectTypeQuery Enum")))
            (if true
              (bind _asbp_player (cast `/Game/Blueprints/BP_Player` (`.HitActor` (`GameplayStatics.BreakHitResult` _outhit))))
              (`/Game/Blueprints/BP_PlayerStats.DecreaseSanity` _asbp_player (`self.AttackDamage`))
              (`KismetSystemLibrary.Delay` 0.2)
              (`self.Process Array`))))
        (else
          (bind _result (`/Engine/EditorBlueprintResources/StandardMacros.IncrementInt` _currentwaypoint)
            (:`  `
              (if (< _result (`KismetArrayLibrary.Array_Length` _waypoints))
                (set `self.CurrentWayPoint` _result)
                (`KismetSystemLibrary.Delay` 0.2)
                (`self.Process Array`)
                (else
                  (set `self.CurrentWayPoint` 0)
                  (`KismetSystemLibrary.Delay` 0.2)
                  (`self.Process Array`))))))))))

(event `self.Start Shot`
  (`self.K2_DestroyActor`))

(fn `UserConstructionScript`)