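; PuzzleManager runs a chime sequence puzzle that opens a door.
; SubmitChime appends each chime ID to PlayerSequence and, while unsolved, loops over it and compares an entry with Sequence at the same index.
; A match immediately sets the solved flag and calls OpenDoor on DoorRef, with no check for full sequence length.
; A mismatch clears the player's input and prints a wrong-code message.
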(fn `SubmitChime`
  (params (ChimeID :type Integer))
  (`KismetArrayLibrary.Array_Add` (`self.PlayerSequence`) ChimeID)
  (if (== (`self.bpPuzzleSolved`) false)
    (for (_array_element _array_index) (`self.PlayerSequence`) :!label _label
      _)
    (if (== _array_element (`|GetArrayItem` (`self.Sequence`) _array_index))
      (set `self.bpPuzzleSolved` true)
      (`/Game/Blueprints/BP_SoE/Door.OpenDoor` (`self.DoorRef`))
      (else
        (`KismetArrayLibrary.Array_Clear` (`self.PlayerSequence`))
        (`KismetSystemLibrary.PrintString` "WrongCode")
        (goto _label :!via `Break`)))))

(fn `UserConstructionScript`)