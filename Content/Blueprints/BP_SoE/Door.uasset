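; Door actor that opens when the player's chime sequence puzzle is solved.
; It finds the PuzzleManager in the level at BeginPlay.
; TryOpen submits the chime to the manager, then either opens the door or resets the manager's sequence on failure.
; Opening snaps the actor to a 90-degree relative rotation on one axis and prints a debug message.
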(event `self.ReceiveBeginPlay`
  (bind _returnvalue (`GameplayStatics.GetActorOfClass` "/Game/Blueprints/BP_SoE/PuzzleManager.PuzzleManager_C"))
  (set `self.PuzzleManagerRef` _returnvalue))

(event `TryOpen`
  (bind _puzzlemanagerref (`self.PuzzleManagerRef`))
  (bind _true (`/Game/Blueprints/BP_SoE/PuzzleManager.SubmitChime` _puzzlemanagerref))
  (if _true
    (`self.OpenDoor`)
    (else
      (`/Game/Blueprints/BP_SoE/PuzzleManager.ResetSeq` _puzzlemanagerref))))

(event `OpenDoor`
  (`KismetSystemLibrary.PrintString` "Correct")
  (`self.K2_SetActorRelativeRotation` (struct :`Yaw` 90.0)))

(fn `UserConstructionScript`)