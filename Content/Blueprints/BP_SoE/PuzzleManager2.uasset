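; PuzzleManager2 manages a chime puzzle in which played strings are checked against a target sequence.
; StringPlayed appends each string ID to PlayerSequence and prints a debug "Hello", while ResetSeq clears that array.
; SubmitChime returns whether PlayerSequence is identical to Sequence, without resetting it or triggering any outcome itself.
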(event `StringPlayed`
  (params (StringID :type Integer))
  (`KismetSystemLibrary.PrintString` "Hello")
  (`KismetArrayLibrary.Array_Add` (`self.PlayerSequence`) StringID))

(event `ResetSeq`
  (`KismetArrayLibrary.Array_Clear` (`self.PlayerSequence`)))

(fn `SubmitChime`
  (returns (True :type Boolean))
  (return (`KismetArrayLibrary.Array_Identical` (`self.Sequence`) (`self.PlayerSequence`))))

(fn `UserConstructionScript`)