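; Small cave door actor that opens when the puzzle sequence is submitted correctly.
; It finds the PuzzleManager2 actor at BeginPlay, and TryOpen asks it to validate the submission via SubmitString.
; Success prints a confirmation and snaps the door to a fixed relative rotation with no animation, while failure resets the manager's sequence.
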(event `self.ReceiveBeginPlay`
  (bind _returnvalue (`GameplayStatics.GetActorOfClass` "/Game/Blueprints/BP_SoE/PuzzleManager2.PuzzleManager2_C"))
  (set `self.PuzzleManagerRef` _returnvalue))

(event `TryOpen`
  (bind _puzzlemanagerref (`self.PuzzleManagerRef`))
  (bind _true (`/Game/Blueprints/BP_SoE/PuzzleManager2.SubmitString` _puzzlemanagerref))
  (if _true
    (`self.OpenDoor`)
    (else
      (`/Game/Blueprints/BP_SoE/PuzzleManager2.ResetSeq` _puzzlemanagerref))))

(event `OpenDoor`
  (`KismetSystemLibrary.PrintString` "Correct")
  (`self.K2_SetActorRelativeRotation` (struct :`Yaw` 150.0)))

(fn `UserConstructionScript`)